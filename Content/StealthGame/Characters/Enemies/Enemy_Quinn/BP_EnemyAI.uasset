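; Stealth-game enemy AI that patrols, chases the player on sight and melee attacks, sending a hit player back to checkpoint.
; Tick drives AIMoveTo chasing or patrolling, either looping target points or one random move that never re-enables CanMove.
; PawnSensing sets visibility, cleared by a one-second retriggerable delay with material swaps, and sends the enemy toward noises.
; A montage notify triggers the hand-socket sphere trace; misses re-arm the attack.
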(event OnSeePawn(PawnSensing)
  (params (Pawn :type Pawn%20Object%20Reference))
  (Utilities|FlowControl|Sequence
    (:then_0
      (Utilities|Casting|CastToBP_ThirdPersonCharacterCustom Pawn
        (:then
          (Development|PrintString "Hey! Stop right there!" true true "(R=0.990625,G=0.000000,B=0.010944,A=1.000000)")
          (Rendering|Material|SetMaterial (Variables|Character|GetMesh) 0 "/Engine/EngineDebugMaterials/ShadedLevelColorationUnlitMateri.ShadedLevelColorationUnlitMateri")
          ;[1 0 0.01552 0.5] Remember to turn this on for chasing
          (Variables|Default|SetbPlayerVisible true))
        (:CastFailed
          (Variables|Default|SetbPlayerVisible false))))
    (:then_1
      (Utilities|FlowControl|RetriggerableDelay 1.0)
      (Variables|Default|SetbPlayerVisible false)
      (Development|PrintString "Must've been the wind....." true true "(R=0.000000,G=0.052961,B=1.000000,A=1.000000)")
      (Rendering|Material|SetMaterial (Variables|Character|GetMesh) 0 "/Engine/EngineDebugMaterials/VertexColorViewMode_GreenOnly.VertexColorViewMode_GreenOnly"))))

(event OnHearNoise(PawnSensing)
  (params (Instigator :type Pawn%20Object%20Reference) (Location :type Vector%20%28by%20ref%29 :default "0, 0, 0") (Volume :type Float%20%28single-precision%29))
  (CallFunction|UpdateWalkSpeed 2e+02)
  (Variables|Default|SetbCanMove false)
  (AI|AIMoveTo self Location Instigator 5e+01 false
    (:OnSuccess
      (Utilities|FlowControl|Delay 12.0)
      (Variables|Default|SetbCanMove true))))

(event Custom|ChasePlayer
  (CallFunction|UpdateWalkSpeed 4.5e+02)
  (Variables|Default|SetbCanMove false)
  (AI|AIMoveTo self "0, 0, 0" (Game|GetPlayerCharacter 0) 75.0 false
    (:OnSuccess
      (CallFunction|Attack))))

(event Custom|Attack
  (bind _mesh (Variables|Character|GetMesh))
  (bind _returnvalue (Transformation|GetSocketLocation _mesh "hand_r"))
  ;[0.15 0.1407 0.04319 0.5] Bonk
  (Utilities|FlowControl|DoOnce false ; Only Reset Attack on miss.
    (:Completed
      (bind _notifyname (Animation|Montage|PlayMontage (Variables|Character|GetMesh) "/Game/StealthGame/Characters/Enemies/AM_Attack_01.AM_Attack_01") ; Play the AM_Attack_01
        (:OnCompleted
          (if (Variables|Default|GetbHostile) ; Keep attacking if you haven't landed the hit.
            (CallFunction|ResetAttack)))
        (:OnNotifyBegin
          (switch name _notifyname ; Pick the proper attack type(standard when there is more than one type of attack)
            (:AttackDamage
              (Development|PrintString "I'm attacking!")
              (bind (_outhits _returnvalue_2) (Collision|MultiSphereTraceForObjects _returnvalue (+ _returnvalue (* (Transformation|GetActorForwardVector) (Variables|Default|GetMeleeTraceDistance))) (Variables|Default|GetMeleeTraceRadius) (Utilities|Array|MakeArray "ObjectTypeQuery3") false 0 "ForDuration")) ; Trace forward from hand socket.
              (if _returnvalue_2 ; If a pawn is hit in that trace...
                (for _array_element _outhits ; ...loop through the results....
                  (bind _asbp_third_person_character_custom (Utilities|Casting|CastToBP_ThirdPersonCharacterCustom (.HitActor (Collision|BreakHitResult _array_element))))
                  (Default|LoadCheckpoint _asbp_third_person_character_custom)
                  (Variables|Default|SetbHostile false) ; ...and stop attacking...
                )))))))))

(event Custom|MoveToNextPatrolPoints
  (Rendering|Material|SetMaterial (Variables|Character|GetMesh) 0 "/Engine/EngineDebugMaterials/VertexColorViewMode_GreenOnly.VertexColorViewMode_GreenOnly")
  (CallFunction|UpdateWalkSpeed 2e+02)
  (Variables|Default|SetbCanMove false)
  (AI|AIMoveTo self "0, 0, 0" (Utilities|Array|Get(acopy) (Variables|Default|GetTargetPoints) (Variables|Default|GetPatrolTargetPointIndex)) 5.0 false
    (:OnSuccess
      (CallFunction|SetNextPatrolPointIndex)
      (Utilities|FlowControl|Delay 1.0)
      (Variables|Default|SetbCanMove true))))

(event Custom|ResetAttack
  (bind _mesh (Variables|Character|GetMesh))
  (bind _returnvalue (Transformation|GetSocketLocation _mesh "hand_r"))
  ;[0.15 0.1407 0.04319 0.5] Bonk
  (Utilities|FlowControl|DoOnce false) ; enters at Reset
)

(event Custom|PatrolRandom
  (Rendering|Material|SetMaterial (Variables|Character|GetMesh) 0 "/Engine/EngineDebugMaterials/VertexColorViewMode_GreenOnly.VertexColorViewMode_GreenOnly")
  (CallFunction|UpdateWalkSpeed 2e+02)
  (Variables|Default|SetbCanMove false)
  (AI|AIMoveTo self (.RandomLocation (AI|Navigation|GetRandomReachablePointinRadius (Transformation|GetActorLocation) 2e+03 0 0)) 0 75.0 false
    (:OnSuccess
      (Utilities|FlowControl|Delay 3.0)
      (Variables|Default|SetbCanMove false))))

(event Custom|SetNextPatrolPointIndex
  (Variables|Default|SetPatrolTargetPointIndex (Math|Integer|%(Integer) (+ (Variables|Default|GetPatrolTargetPointIndex) 1) (Utilities|Array|Length (Variables|Default|GetTargetPoints)))))

(event EventBeginPlay)

(event Collision|EventActorBeginOverlap
  (params (OtherActor :type Actor%20Object%20Reference)))

(event EventTick
  (params (DeltaSeconds :type Float%20%28single-precision%29))
  (bind _bplayervisible (Variables|Default|GetbPlayerVisible))
  (if (Variables|Default|GetbCanMove)
    (if _bplayervisible
      (CallFunction|ChasePlayer)
      (elif (Variables|Default|GetbTargetPonintMovement)
        (CallFunction|MovetoNextPatrolPoints)
        (else
          (CallFunction|PatrolRandom))))
    (elif _bplayervisible
      (CallFunction|ChasePlayer))))

(fn ConstructionScript)

(fn UpdateWalkSpeed
  (params (NewWalkSpeed :type Float%20%28double-precision%29))
  (Variables|/Script/Engine.CharacterMovementComponent|SetMaxWalkSpeed (Variables|Character|GetCharacterMovement) NewWalkSpeed))